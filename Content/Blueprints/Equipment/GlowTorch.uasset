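; GlowTorch is an equipment Blueprint for a torch that becomes a physics object when the RuthCharacter first touches it.
; BeginPlay stores the Torch component in StaticMeshObject.
; The Torch's begin-overlap event enables physics simulation once, gated by a DoOnce boolean, and ignores overlapping components whose first tag is "Targetting".
; Tick and the construction script are empty.
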(event `self.ReceiveBeginPlay`
  (set `self.StaticMeshObject` (`self.Torch`)))

(event `self.Torch.OnComponentBeginOverlap`
  (params (OverlappedComponent :type "PrimitiveComponent Object Reference") (OtherActor :type "Actor Object Reference") (OtherComp :type "PrimitiveComponent Object Reference") (OtherBodyIndex :type Integer) (bFromSweep :type Boolean) (SweepResult :type "HitResult Structure (by ref)"))
  (if (`self.DoOnce`)
    (if (and (`KismetMathLibrary.ClassIsChildOf` (`GameplayStatics.GetObjectClass` OtherActor) "/Game/Blueprints/Characters/RuthCharacter.RuthCharacter_C") (!= (`KismetArrayLibrary.Array_Get` (`ActorComponent.ComponentTags` OtherComp)) "Targetting"))
      (`PrimitiveComponent.SetSimulatePhysics` (`self.Torch`) true)
      (set `self.DoOnce` false))))

(event `self.ReceiveTick`
  (params (DeltaSeconds :type "Float (single-precision)")))

(fn `UserConstructionScript`)
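; LabCam is a shared multiplayer camera that becomes the view target and follows the average location of all RuthTestCharacter actors.
; Tick plays a timeline that lerps the AverageLocation component toward that point and adjusts minimum zoom by player count and farthest player distance from the camera actor.
; When the timeline finishes, spring arm length becomes twice the first player's distance from the average, clamped to zoom limits, and dead players are dropped.
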(event `self.ReceiveBeginPlay`
  (`KismetSystemLibrary.Delay` 0.0)
  (bind _outactors (`GameplayStatics.GetAllActorsOfClass` "/Script/ToyBoxBrawl.RuthTestCharacter"))
  (bind _output_get (set `self.Players` _outactors))
  (`PlayerController.SetViewTargetWithBlend` (`GameplayStatics.GetPlayerController` 0) self 0.0 "VTBlend_Linear" 0.0 false)
  (bind _returnvalue (`GameplayStatics.GetActorArrayAverageLocation` _output_get))
  (set `SpringArmComponent.TargetArmLength` (`KismetMathLibrary.FClamp` (* (`KismetMathLibrary.VSize` (- _returnvalue (`self.K2_GetActorLocation` (`KismetArrayLibrary.Array_Get` _output_get)))) 2.0) (`self.MinZoom`) (`self.MaxZoom`)) (`self.SpringArm`))
  (`SceneComponent.K2_SetWorldLocation` (`self.AverageLocation`) _returnvalue false true))

(event `self.ReceiveTick`
  (params (DeltaSeconds :type "Float (single-precision)"))
  (bind _averagelocation (`self.AverageLocation`))
  (bind _players (`self.Players`))
  (bind _returnvalue (`GameplayStatics.GetActorArrayAverageLocation` _players))
  (bind (_direction _time) (`Timeline|LerpTimeLine`)
    (:`Update`
      (`SceneComponent.K2_SetWorldLocation` _averagelocation (`KismetMathLibrary.VLerp` (`SceneComponent.K2_GetComponentLocation` _averagelocation) _returnvalue _time) true false)
      (bind _highest_length (`self.FurthestfromAverage`))
      (switch `int` (`KismetArrayLibrary.Array_Length` _players) :!label _label
        (:`2`
          (set `self.DistanceMultipler` 2.0)
          (set `self.MinZoom` 500.0))
        (:`3`
          (set `self.DistanceMultipler` 2.0)
          (bind _returnvalue_2 (`KismetMathLibrary.FClamp` _highest_length 500.0 1100.0))
          (set `self.MinZoom` _returnvalue_2))
        (:`4`
          (set `self.DistanceMultipler` 2.0)
          (set `self.MinZoom` _returnvalue_2))))
    (:`Finished`
      (bind _output_get (set `SpringArmComponent.TargetArmLength` (`KismetMathLibrary.FClamp` (* (`KismetMathLibrary.VSize` (- _returnvalue (`self.K2_GetActorLocation` (`KismetArrayLibrary.Array_Get` _players)))) 2.0) (`self.MinZoom`) (`self.MaxZoom`)) (`self.SpringArm`)))
      (for _array_element _players
        (if (`RuthTestCharacter.bIsDead` _array_element)
          (`KismetArrayLibrary.Array_RemoveItem` (`self.Players`) _array_element)
          (goto _label))))))

(fn `FurthestfromAverage`
  (returns (`Highest Length` :type "Float (double-precision)"))
  (set `self.Highlength` 0.0)
  (for _array_element (`self.Players`)
    (bind _returnvalue (`KismetMathLibrary.VSize` (- (`self.K2_GetActorLocation`) (`self.K2_GetActorLocation` _array_element))))
    (if (> _returnvalue (`self.Highlength`))
      (bind _output_get (set `self.Highlength` _returnvalue))))
  (return (* _output_get (`self.DistanceMultipler`))))

(fn `UserConstructionScript`)
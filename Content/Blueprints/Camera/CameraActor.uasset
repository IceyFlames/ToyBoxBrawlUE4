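; Shared camera actor that tracks the average position of all RuthTestCharacter players along the X axis.
; BeginPlay waits a frame for the players to spawn, then caches them.
; Tick restarts a timeline whose updates lerp the scene component toward the average X at fixed Y and Z, only while that average lies within XBounds.
; NormaliseYZaxis is unused and only prints the farthest player's distance from the average.
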(event EventBeginPlay
  ;[0.1093 0.5715 1] Get all the players, we delay for a frame because the camera is created before the players a frame later.
  (Utilities|FlowControl|Delay 0.0)
  (bind _outactors (Actor|GetAllActorsOfClass "/Script/ToyBoxBrawl.RuthTestCharacter"))
  (Variables|Default|SetPlayers _outactors))

(event EventTick
  (params (DeltaSeconds :type Float%20%28single-precision%29))
  (bind _time (Timeline|Timeline_0 PlayFromStart)
    (:Update
      (CallFunction|NormaliseXaxis _time))))

(fn ConstructionScript)

(fn NormaliseXaxis
  (params (Time :type Float%20%28single-precision%29))
  (bind _scenecomponent (Variables|Default|GetSceneComponent))
  (bind _xbounds (Variables|Default|GetXBounds))
  (bind (_x _y) (Math|Vector2D|BreakVector2D _xbounds))
  (bind _returnvalue (Class|GameplayStatics|GetActorArrayAverageLocation (Variables|Default|GetPlayers)))
  (if (and (< (.X (Math|Vector|BreakVector _returnvalue)) _y) (> (.X (Math|Vector|BreakVector _returnvalue)) _x))
    (Transformation|SetWorldLocation _scenecomponent (Math|Vector|Lerp(Vector) (Transformation|GetWorldLocation _scenecomponent) (Math|Vector|MakeVector (.X (Math|Vector|BreakVector _returnvalue)) 908.934082 623.210815) Time) false false)))

(fn NormaliseYZaxis
  (params (Time :type Float%20%28single-precision%29))
  (bind _players (Variables|Default|GetPlayers))
  (bind _returnvalue (Class|GameplayStatics|GetActorArrayAverageLocation _players))
  (for _array_element _players
    (if (not (> (LocalVariables|GetLengthProduct) (Math|Vector|VectorLength (- _returnvalue (Transformation|GetActorLocation _array_element)))))
      (LocalVariables|SetLengthProduct (Math|Vector|VectorLength (- _returnvalue (Transformation|GetActorLocation _array_element))))))
  (Development|PrintString (Utilities|String|ToString(Float) (LocalVariables|GetLengthProduct))))
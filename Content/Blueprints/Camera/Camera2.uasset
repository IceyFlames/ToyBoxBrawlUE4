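; Shared camera actor that frames all RuthTestCharacter players and becomes player 0's view target at BeginPlay.
; Tick computes the players' average location and plays a timeline that lerps the AverageLocation component toward it with sweep.
; When the timeline finishes, spring arm length is set to twice the first player's distance from that average, clamped between MinZoom and MaxZoom.
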(event `self.ReceiveBeginPlay`
  (`KismetSystemLibrary.Delay` 0.0)
  (bind _outactors (`GameplayStatics.GetAllActorsOfClass` "/Script/ToyBoxBrawl.RuthTestCharacter"))
  (set `self.Players` _outactors)
  (`PlayerController.SetViewTargetWithBlend` (`GameplayStatics.GetPlayerController` 0) self 0.0 "VTBlend_Linear" 0.0 false))

(event `self.ReceiveTick`
  (params (DeltaSeconds :type "Float (single-precision)"))
  (bind _players (`self.Players`))
  (bind _averagelocation (`self.AverageLocation`))
  (bind _returnvalue (`GameplayStatics.GetActorArrayAverageLocation` _players))
  (bind (_direction _time) (`Timeline|LerpTimeLine`)
    (:`Update`
      (`SceneComponent.K2_SetWorldLocation` _averagelocation (`KismetMathLibrary.VLerp` (`SceneComponent.K2_GetComponentLocation` _averagelocation) _returnvalue _time) true false))
    (:`Finished`
      (bind _output_get (set `SpringArmComponent.TargetArmLength` (`KismetMathLibrary.FClamp` (* (`KismetMathLibrary.VSize` (- _returnvalue (`self.K2_GetActorLocation` (`KismetArrayLibrary.Array_Get` _players)))) 2.0) (`self.MinZoom`) (`self.MaxZoom`)) (`self.SpringArm`))))))

(fn `UserConstructionScript`)
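; BeachCam is a shared camera that becomes player 0's view target and frames all RuthTestCharacter actors.
; Each tick it plays a timeline that lerps the AverageLocation component toward the players' average position, clamped per axis.
; When the timeline finishes, spring arm length is set to twice the first player's distance from that average, within zoom limits, and dead players are dropped from tracking.
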(event `self.ReceiveBeginPlay`
  (`KismetSystemLibrary.Delay` 0.0)
  (bind _outactors (`GameplayStatics.GetAllActorsOfClass` "/Script/ToyBoxBrawl.RuthTestCharacter"))
  (bind _output_get (set `self.Players` _outactors))
  (`PlayerController.SetViewTargetWithBlend` (`GameplayStatics.GetPlayerController` 0) self 0.0 "VTBlend_Linear" 0.0 false)
  (bind _returnvalue (`GameplayStatics.GetActorArrayAverageLocation` _output_get))
  (set `SpringArmComponent.TargetArmLength` (`KismetMathLibrary.FClamp` (* (`KismetMathLibrary.VSize` (- _returnvalue (`self.K2_GetActorLocation` (`KismetArrayLibrary.Array_Get` _output_get)))) 2.0) (`self.MinZoom`) (`self.MaxZoom`)) (`self.SpringArm`))
  (`SceneComponent.K2_SetWorldLocation` (`self.AverageLocation`) _returnvalue false true))

(event `self.ReceiveTick`
  (params (DeltaSeconds :type "Float (single-precision)"))
  (bind _averagelocation (`self.AverageLocation`))
  (bind _players (`self.Players`))
  (bind _returnvalue (`GameplayStatics.GetActorArrayAverageLocation` _players))
  (bind (_direction _time) (`Timeline|LerpTimeLine`)
    (:`Update`
      (`SceneComponent.K2_SetWorldLocation` _averagelocation (`KismetMathLibrary.MakeVector` (`KismetMathLibrary.FClamp` (.x (`KismetMathLibrary.VLerp` (`SceneComponent.K2_GetComponentLocation` _averagelocation) _returnvalue _time)) (`self.MinXpos`) (`self.MaxXpos`)) (`KismetMathLibrary.FClamp` (.y (`KismetMathLibrary.VLerp` (`SceneComponent.K2_GetComponentLocation` _averagelocation) _returnvalue _time)) (`self.MinYpos`) (`self.MaxYpos`)) (`KismetMathLibrary.FClamp` (.z (`KismetMathLibrary.VLerp` (`SceneComponent.K2_GetComponentLocation` _averagelocation) _returnvalue _time)) (`self.MinZPos`) (`self.MaxZPos`))) true false))
    (:`Finished`
      (bind _output_get (set `SpringArmComponent.TargetArmLength` (`KismetMathLibrary.FClamp` (* (`KismetMathLibrary.VSize` (- _returnvalue (`self.K2_GetActorLocation` (`KismetArrayLibrary.Array_Get` _players)))) 2.0) (`self.MinZoom`) (`self.MaxZoom`)) (`self.SpringArm`)))
      (for _array_element _players
        (if (`RuthTestCharacter.bIsDead` _array_element)
          (`KismetArrayLibrary.Array_RemoveItem` (`self.Players`) _array_element))))))

(fn `UserConstructionScript`)
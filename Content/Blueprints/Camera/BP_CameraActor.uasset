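; Shared camera actor that follows the average location of all RuthTestCharacter players, gathered one frame after BeginPlay because they spawn later.
; Each tick it lerps the camera using a clamped ZoomPercent as both offset scale and alpha, then clamps the world position's vector length.
; CalculateHighestPoint then feeds the next move with the farthest player distance for zoom and a height offset (highest Z minus average-location Y).
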(event EventBeginPlay
  ;[0.1093 0.5715 1] Get all the players, we delay for a frame because the camera is created before the players a frame later.
  (Utilities|FlowControl|Delay 0.0)
  (bind _outactors (Actor|GetAllActorsOfClass "/Script/ToyBoxBrawl.RuthTestCharacter"))
  (Variables|Default|SetPlayers _outactors))

(event EventTick
  (params (DeltaSeconds :type Float%20%28single-precision%29))
  (CallFunction|LerpXYZAxis)
  (CallFunction|CalculateHighestPoint))

(fn ConstructionScript)

(fn LerpXYZAxis
  (bind _cameracomponent (Variables|CameraActor|GetCameraComponent))
  (bind _returnvalue (Class|GameplayStatics|GetActorArrayAverageLocation (Variables|Default|GetPlayers)))
  (Variables|Default|SetAvgLocation _returnvalue)
  (bind _output_get (Variables|Default|SetZoomPercent (/ (Variables|Default|GetLengthProduct) 4e+02)))
  (Variables|Default|SetZoomPercent (Math|Float|Clamp(Float) _output_get 0.75 1.1))
  (Transformation|SetWorldLocation _cameracomponent (Math|Vector|ClampVectorSize (Math|Vector|Lerp(Vector) (Transformation|GetWorldLocation _cameracomponent) (Math|Vector|MakeVector (.X (Math|Vector|BreakVector _returnvalue)) (.Y (Math|Vector|BreakVector (* (- (Transformation|GetActorLocation) _returnvalue) (Variables|Default|GetZoomPercent)))) (+ (.Z (Math|Vector|BreakVector (* (- (Transformation|GetActorLocation) _returnvalue) (Variables|Default|GetZoomPercent)))) (Variables|Default|GetHighestPoint))) (Variables|Default|GetZoomPercent)) 6.8e+02 1.2e+03) false false))

(fn CalculateHighestPoint
  (Transformation|SetWorldLocation (Variables|Default|GetAverageLocation) (Variables|Default|GetAvgLocation) true false)
  (for _array_element (Variables|Default|GetPlayers)
    (if (> (LocalVariables|GetTempLength) (Math|Vector|VectorLength (- (Variables|Default|GetAvgLocation) (Transformation|GetActorLocation _array_element))))
      _
      (else
        (bind _output_get (LocalVariables|SetTempLength (Math|Vector|VectorLength (- (Variables|Default|GetAvgLocation) (Transformation|GetActorLocation _array_element)))))
        (Variables|Default|SetLengthProduct _output_get)))
    (if (> (.Z (Math|Vector|BreakVector (Transformation|GetActorLocation _array_element))) (LocalVariables|GetTHighestPoint))
      (bind _output_get_2 (LocalVariables|SetTHighestPoint (.Z (Math|Vector|BreakVector (Transformation|GetActorLocation _array_element)))))
      (Variables|Default|SetHighestPoint (- _output_get_2 (.Y (Math|Vector|BreakVector (Transformation|GetWorldLocation (Variables|Default|GetAverageLocation)))))))))
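; Pawn-side controller that drives gamepad navigation and selection in the main menu.
; It finds the MainMenu widget on BeginPlay, then D-pad presses or analog stick movement, throttled by a Delay, step a wrapping four-option index that updates the widget's position.
; The bottom face button opens the lobby, launches a web form, quits, or adds a preset player to GameInfo and loads the test gameplay level.
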(event `self.ReceiveBeginPlay`
  ;[1 1 1] BeginPlay Stuffs
  (bind _foundwidgets (`WidgetBlueprintLibrary.GetAllWidgetsOfClass` "/Game/Blueprints/Widgets/MainMenu.MainMenu_C"))
  (`/Game/Blueprints/Widgets/MainMenu.SetButtonColour` (cast `/Game/Blueprints/Widgets/MainMenu` (`KismetArrayLibrary.Array_Get` _foundwidgets) :!pure true) (`self.ButtonSelected`) (struct :`R` 0.082283 :`G` 1.0 :`A` 1.0)))

(event `InputAction|Dpad_up`
  (params (Key :type "Key Structure" :default "AnyKey"))
  ;[0.2546 0.114 1] Selecting which button is highlighted
  (:`Pressed`
    (bind _result (`/Engine/EditorBlueprintResources/StandardMacros.DecrementInt` (`self.ButtonSelected`))
      (:`  `
        (if (< _result 0)
          (set `self.ButtonSelected` 3))
        (`/Game/Blueprints/Widgets/MainMenu.SetControllerUIPosition` (cast `/Game/Blueprints/Widgets/MainMenu` (`KismetArrayLibrary.Array_Get` (stale `self.ReceiveBeginPlay` _foundwidgets)) :!pure true) (stale `InputAction|Dpad_down` _output_get) :!label _label)))))

(event `InputAction|Dpad_down`
  (params (Key :type "Key Structure" :default "AnyKey"))
  ;[0.2546 0.114 1] Selecting which button is highlighted
  (:`Pressed`
    (bind _result (`/Engine/EditorBlueprintResources/StandardMacros.IncrementInt` (`self.ButtonSelected`))
      (:`  `
        (if (> _result 3)
          (bind _output_get (set `self.ButtonSelected` 0))
          (goto _label)
          (else
            (goto _label)))))))

(event `InputAction|Bottom_Button`
  (params (Key :type "Key Structure" :default "AnyKey"))
  (:`Pressed`
    (switch `int` (`self.ButtonSelected`)
      (:`0`
        (`GameplayStatics.OpenLevel` "LobbyMap"))
      (:`1`
        (`KismetSystemLibrary.LaunchURL` "https://goo.gl/forms/a5dmGka7uRzmLCqn2"))
      (:`2`
        (`KismetSystemLibrary.QuitGame` null "Quit"))
      (:`3`
        (`KismetArrayLibrary.Array_AddUnique` (`GameInstanceTBB._TPlayers` (cast `/Game/Blueprints/GameInstance/GameInfo` (`GameplayStatics.GetGameInstance`) :!pure true)) (make `PlayerCharacter` 0 "Ruth" 1 1))
        (`GameplayStatics.OpenLevel` "TestGameplay")))))

(event `InputAxis|MoveForward`
  (params (AxisValue :type "Float (single-precision)"))
  (bind _buttonselected (`self.ButtonSelected`))
  ;[1 0 0.5417] Analog Support
  (`KismetSystemLibrary.Delay` 0.15)
  (if (> AxisValue 0.3)
    (bind _result (`/Engine/EditorBlueprintResources/StandardMacros.DecrementInt` _buttonselected)
      (:`  `
        (if (< _result 0)
          (bind _output_get (set `self.ButtonSelected` 3)))
        (`/Game/Blueprints/Widgets/MainMenu.SetControllerUIPosition` (cast `/Game/Blueprints/Widgets/MainMenu` (`KismetArrayLibrary.Array_Get` (stale `self.ReceiveBeginPlay` _foundwidgets)) :!pure true) _output_get :!label _label_2)))
    (elif (< AxisValue -0.3)
      (bind _result_2 (`/Engine/EditorBlueprintResources/StandardMacros.IncrementInt` _buttonselected)
        (:`  `
          (if (> _result_2 3)
            (set `self.ButtonSelected` 0)
            (goto _label_2)
            (else
              (goto _label_2))))))))

(fn `UserConstructionScript`)
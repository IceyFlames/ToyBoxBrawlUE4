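; Lobby pawn that lets a joining player preview a character during character creation.
; The first bottom-button press marks it connected, caches the JoinLobby widget, shows CharacterCreation and loads a default Ruth mesh, looping idle and red hair.
; D-pad up/down wraps through six creation elements unless a HUD element is selected.
; Helper functions swap among three characters and apply hair and body colour materials, but only the hair one is called here.
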(event `InputAction|Bottom_Button`
  (params (Key :type "Key Structure" :default "AnyKey"))
  ;[1 0 0.04459] Selecting Options
  (:`Pressed`
    (if (not (`self.ConnectedtoGame`))
      (bind _output_get (set `self.ConnectedtoGame` true))
      (bind _foundwidgets (`WidgetBlueprintLibrary.GetAllWidgetsOfClass` "/Game/Blueprints/Widgets/JoinLobby.JoinLobby_C" _output_get))
      (set `self.LobbyReference` (cast `/Game/Blueprints/Widgets/JoinLobby` (`KismetArrayLibrary.Array_Get` _foundwidgets) :!pure true))
      (`SceneComponent.SetVisibility` (`self.CharacterCreation`) true false)
      (`self.AssignMeshObjects`)
      (`self.Set Hair Material` 0))))

(event `InputAction|Right_button`
  (params (Key :type "Key Structure" :default "AnyKey"))
  ;[1 0 0.04459] Selecting Options
)

(event `InputAction|Dpad_up`
  (params (Key :type "Key Structure" :default "AnyKey"))
  ;[0.01856 1 0] Dpad Up Input
  (:`Pressed`
    (if (`self.ConnectedtoGame`)
      (if (not (`self.HudElementSelected`))
        (bind _output_get (set `self.CharacterCreationElement` (- (`self.CharacterCreationElement`) 1)))
        (if (< _output_get 0)
          (set `self.CharacterCreationElement` 5))))))

(event `InputAction|Dpad_down`
  (params (Key :type "Key Structure" :default "AnyKey"))
  ;[0 0.3801 1] DpadDown Input
  (:`Pressed`
    (if (`self.ConnectedtoGame`)
      (if (not (`self.HudElementSelected`))
        (bind _output_get (set `self.CharacterCreationElement` (+ (`self.CharacterCreationElement`) 1)))
        (if (> _output_get 5)
          (set `self.CharacterCreationElement` 0))))))

(event `InputAxis|MoveForward`
  (params (AxisValue :type "Float (single-precision)"))
  ;[1 0.1208 0.9433] Analog Stick Support
)

(fn `AssignMeshObjects`
  (bind _skeletalmesh (`self.SkeletalMesh`))
  (`StaticMeshComponent.SetStaticMesh` (`self.Hair`) "/Game/Assets/Models/Accesories/Ruth_hair__2_.Ruth_hair__2_")
  (`SkinnedMeshComponent.SetSkinnedAssetAndUpdate` _skeletalmesh "/Game/Assets/Models/Characters/Ruth/Real_Ruth_UE4.Real_Ruth_UE4")
  (`SkeletalMeshComponent.SetAnimationMode` _skeletalmesh "AnimationSingleNode")
  (`SkeletalMeshComponent.PlayAnimation` _skeletalmesh "/Game/Assets/Animations/Ruth/Ruth_Idle_Anim.Ruth_Idle_Anim" true))

(fn `Set Body Material`
  (params (ColourID :type Integer) (CharacterID :type Integer))
  (bind _skeletalmesh (`self.SkeletalMesh`))
  (bind _skeletalmesh_2 (`self.SkeletalMesh`))
  (switch `int` CharacterID
    (:`0`
      (switch `int` ColourID :!label _label
        (:`0`
          (`PrimitiveComponent.SetMaterial` _skeletalmesh_2 1 "/Game/Assets/Material/Characters/Ruth/RedI.RedI"))
        (:`1`
          (`PrimitiveComponent.SetMaterial` _skeletalmesh_2 1 "/Game/Assets/Material/Characters/Ruth/Blue.Blue"))
        (:`2`
          (`PrimitiveComponent.SetMaterial` _skeletalmesh_2 1 "/Game/Assets/Material/Characters/Ruth/Green.Green"))
        (:`3`
          (`PrimitiveComponent.SetMaterial` _skeletalmesh_2 1 "/Game/Assets/Material/Characters/Ruth/Yellow.Yellow"))
        (:`4`
          (`PrimitiveComponent.SetMaterial` _skeletalmesh_2 1 "/Game/Assets/Material/Characters/Ruth/Purple.Purple")))
      (`PrimitiveComponent.SetMaterial` _skeletalmesh_2 2 "/Game/Assets/Material/Characters/Ruth/ruthFace.ruthFace"))
    (:`1`
      (switch `int` ColourID
        (:`0`
          (`PrimitiveComponent.SetMaterial` _skeletalmesh 2 "/Game/Assets/Material/Characters/Aeiou/AEIOU_RedLimbs_Mat.AEIOU_RedLimbs_Mat"))
        (:`1`
          (`PrimitiveComponent.SetMaterial` _skeletalmesh 2 "/Game/Assets/Material/Characters/Aeiou/AEIOU_BlueLimbs_Mat.AEIOU_BlueLimbs_Mat"))
        (:`2`
          (`PrimitiveComponent.SetMaterial` _skeletalmesh 2 "/Game/Assets/Material/Characters/Aeiou/AEIOU_GreenLimbs_Mat.AEIOU_GreenLimbs_Mat"))
        (:`3`
          (`PrimitiveComponent.SetMaterial` _skeletalmesh 2 "/Game/Assets/Material/Characters/Aeiou/AEIOU_YellowLimbs_Mat.AEIOU_YellowLimbs_Mat"))
        (:`4`
          (`PrimitiveComponent.SetMaterial` _skeletalmesh 2 "/Game/Assets/Material/Characters/Aeiou/AEIOU_PurpleLimbs_Mat.AEIOU_PurpleLimbs_Mat"))))
    (:`2`
      (goto _label))))

(fn `Set Character Mesh`
  (params (`Character Index` :type Integer) (`Connected to game` :type Boolean))
  (bind _skeletalmesh (`self.SkeletalMesh`))
  (bind _hair (`self.Hair`))
  (if `Connected to game`
    (switch `int` `Character Index`
      (:`0`
        (`SkinnedMeshComponent.SetSkinnedAssetAndUpdate` _skeletalmesh "/Game/Assets/Models/Characters/Ruth/Real_Ruth_UE4.Real_Ruth_UE4")
        (`SkeletalMeshComponent.SetAnimationMode` _skeletalmesh "AnimationSingleNode")
        (`SkeletalMeshComponent.PlayAnimation` _skeletalmesh "/Game/Assets/Animations/Ruth/Ruth_Idle_Anim.Ruth_Idle_Anim" true)
        (`StaticMeshComponent.SetStaticMesh` _hair "/Game/Assets/Models/Accesories/Ruth_hair__2_.Ruth_hair__2_"))
      (:`1`
        (`SkinnedMeshComponent.SetSkinnedAssetAndUpdate` _skeletalmesh "/Game/Assets/Models/Characters/AEIOU/UE4_Aeiou.UE4_Aeiou")
        (`SkeletalMeshComponent.SetAnimationMode` _skeletalmesh "AnimationSingleNode")
        (`SkeletalMeshComponent.PlayAnimation` _skeletalmesh "/Game/Assets/Animations/AEIOU/Aeiou_Idle.Aeiou_Idle" true)
        (`StaticMeshComponent.SetStaticMesh` _hair null))
      (:`2`
        (`SkinnedMeshComponent.SetSkinnedAssetAndUpdate` _skeletalmesh "/Game/Assets/Models/Characters/Maniquin/Ruth_UE4.Ruth_UE4")
        (`SkeletalMeshComponent.SetAnimationMode` _skeletalmesh "AnimationSingleNode")
        (`SkeletalMeshComponent.PlayAnimation` _skeletalmesh "/Game/Assets/Animations/Maniquin/RuthIdleAnim.RuthIdleAnim" true)
        (`StaticMeshComponent.SetStaticMesh` _hair null)))
    (else
      (`SkinnedMeshComponent.SetSkinnedAssetAndUpdate` _skeletalmesh null)
      (`SkeletalMeshComponent.SetAnimationMode` _skeletalmesh "AnimationSingleNode")
      (`SkeletalMeshComponent.PlayAnimation` _skeletalmesh null true)
      (`StaticMeshComponent.SetStaticMesh` _hair null))))

(fn `Set Hair Material`
  (params (ColourID :type Integer))
  (bind _hair (`self.Hair`))
  (switch `int` ColourID
    (:`0`
      (`PrimitiveComponent.SetMaterial` _hair 0 "/Game/Assets/Material/Characters/Ruth/RedI.RedI"))
    (:`1`
      (`PrimitiveComponent.SetMaterial` _hair 0 "/Game/Assets/Material/Characters/Ruth/Blue.Blue"))
    (:`2`
      (`PrimitiveComponent.SetMaterial` _hair 0 "/Game/Assets/Material/Characters/Ruth/Green.Green"))
    (:`3`
      (`PrimitiveComponent.SetMaterial` _hair 0 "/Game/Assets/Material/Characters/Ruth/Yellow.Yellow"))
    (:`4`
      (`PrimitiveComponent.SetMaterial` _hair 0 "/Game/Assets/Material/Characters/Ruth/Purple.Purple"))
    (:`5`
      (`PrimitiveComponent.SetMaterial` _hair 0 "/Game/Assets/Material/Characters/Ruth/Brown.Brown"))
    (:`6`
      (`PrimitiveComponent.SetMaterial` _hair 0 "/Game/Assets/Material/Characters/Ruth/Black.Black"))
    (:`7`
      (`PrimitiveComponent.SetMaterial` _hair 0 "/Game/Assets/Material/Characters/Ruth/Orange.Orange"))))

(fn `UserConstructionScript`)
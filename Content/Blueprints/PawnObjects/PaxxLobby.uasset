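; Lobby pawn for one controller that previews and picks a player's character, Ruth or AEIOU.
; Bottom button joins, then readies up, adding the player struct to GameInfo's TPlayers; right button un-readies or leaves.
; D-pad and stick cycle characters, swapping meshes and randomizing hair and body materials, with colours mirrored to the JoinLobby widget.
; Start does nothing, and the level-open and player-removal nodes are disconnected.
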(event `InputAction|Pause`
  (params (Key :type "Key Structure" :default "AnyKey"))
  ;[1 1 1] Start is Pressed to initiate game
  (:`Pressed`
    (if (and (`self.HairColourSelected`) (> (`KismetArrayLibrary.Array_Length` (`GameInstanceTBB._TPlayers` (cast `/Game/Blueprints/GameInstance/GameInfo` (`GameplayStatics.GetGameInstance`) :!pure true))) 1))
      _)))

(event `InputAction|Bottom_Button`
  (params (Key :type "Key Structure" :default "AnyKey"))
  (bind _controllerid (`self.ControllerID`))
  ;[0.08708 0 1] Selecting Options
  (:`Pressed`
    (if (`self.ConnectedtoGame`)
      (set `self.CharacterSelected` true)
      (bind _asjoin_lobby (cast `/Game/Blueprints/Widgets/JoinLobby` (`KismetArrayLibrary.Array_Get` (stale _foundwidgets)) :!pure true))
      (`/Game/Blueprints/Widgets/JoinLobby.SetReadyTextVisible` _asjoin_lobby (`self.ControllerID`) true)
      (switch `int` (`self.CharacterIndexValue`)
        (:`0`
          (set `self.CharacterName` "Ruth"))
        (:`1`
          (set `self.CharacterName` "AEIOU"))
        (:`2`
          (bind _output_get (set `self.CharacterName` "Ruth"))))
      (bind _output_get_2 (set `self.PlayerStructure` (make `PlayerCharacter` (`self.ControllerID`) _output_get (`self.BodyIndexValue`) (`self.HairIndexValue`))))
      (`KismetArrayLibrary.Array_AddUnique` (`GameInstanceTBB._TPlayers` (cast `/Game/Blueprints/GameInstance/GameInfo` (`GameplayStatics.GetGameInstance`) :!pure true)) _output_get_2)
      (else
        (set `self.ConnectedtoGame` true)
        (bind _foundwidgets (`WidgetBlueprintLibrary.GetAllWidgetsOfClass` "/Game/Blueprints/Widgets/JoinLobby.JoinLobby_C"))
        (`self.AssignMeshObjects`)
        (bind _output_get_3 (set `self.HairIndexValue` (`KismetMathLibrary.RandomInteger` 7)))
        (bind _output_get_4 (set `self.BodyIndexValue` (`KismetMathLibrary.RandomInteger` 4)))
        (`self.Set Hair Material` _output_get_3)
        (`self.Set Body Material` _output_get_4 (`self.CharacterIndexValue`))
        (`/Game/Blueprints/Widgets/JoinLobby.SetHairColourUI` _asjoin_lobby _controllerid (stale `InputAction|Dpad_up` _output_get_3) :!label _label)
        (`/Game/Blueprints/Widgets/JoinLobby.SetTorsoColourUI` _asjoin_lobby _controllerid (stale `InputAction|Dpad_up` _output_get_4))))))

(event `InputAction|Right_button`
  (params (Key :type "Key Structure" :default "AnyKey"))
  ;[0.08708 0 1] Selecting Options
  (:`Pressed`
    (if (`self.CharacterSelected`)
      (set `self.CharacterSelected` false)
      (set `self.HairIndexValue` 0)
      (set `self.BodyIndexValue` 0)
      (set `self.CharacterIndexValue` 0)
      (else
        (if (`self.ConnectedtoGame`)
          _
          (else
            _))
        (set `self.ConnectedtoGame` false)
        (`self.UnassignMeshObjects`)
        (set `self.HairIndexValue` 0)
        (set `self.BodyIndexValue` 0)
        (set `self.CharacterIndexValue` 0)))))

(event `InputAction|Dpad_up`
  (params (Key :type "Key Structure" :default "AnyKey"))
  (bind _characterindexvalue (`self.CharacterIndexValue`))
  ;[1 0.4152 0] Dpad Up Input
  (:`Pressed`
    (if (not (`self.ConnectedtoGame`))
      (`self.Set Character Mesh` _characterindexvalue))
    (if (not (`self.CharacterSelected`))
      (bind _output_get (set `self.CharacterIndexValue` (+ _characterindexvalue 1)))
      (if (> _output_get 1)
        (bind _output_get_2 (set `self.CharacterIndexValue` 0)))
      (`self.Set Character Mesh` _output_get_2 true)
      (bind _output_get_3 (set `self.HairIndexValue` (`KismetMathLibrary.RandomInteger` 7)))
      (bind _output_get_4 (set `self.BodyIndexValue` (`KismetMathLibrary.RandomInteger` 4)))
      (`self.Set Hair Material` _output_get_3)
      (`self.Set Body Material` _output_get_4 (`self.CharacterIndexValue`))
      (goto _label))))

(event `InputAction|Dpad_down`
  (params (Key :type "Key Structure" :default "AnyKey"))
  (bind _characterindexvalue (`self.CharacterIndexValue`))
  ;[0.7913 0.016 1] DpadDown Input
  (:`Pressed`
    (if (`self.ConnectedtoGame`)
      (if (not (`self.CharacterSelected`))
        (bind _output_get (set `self.CharacterIndexValue` (- _characterindexvalue 1)))
        (if (< _output_get 0)
          (bind _output_get_2 (set `self.CharacterIndexValue` 1)))
        (`self.Set Character Mesh` _output_get_2 true)
        (bind _output_get_3 (set `self.HairIndexValue` (`KismetMathLibrary.RandomInteger` 7)))
        (bind _output_get_4 (set `self.BodyIndexValue` (`KismetMathLibrary.RandomInteger` 4)))
        (`self.Set Hair Material` _output_get_3)
        (`self.Set Body Material` _output_get_4 (`self.CharacterIndexValue`))
        (goto _label))
      (else
        (`self.Set Character Mesh` _characterindexvalue)))))

(event `InputAxis|MoveForward`
  (params (AxisValue :type "Float (single-precision)"))
  ;[1 1 1] Analog Stick Support
  (`KismetSystemLibrary.Delay` 0.15)
  (if (`self.ConnectedtoGame`)
    (if (> AxisValue 0.3)
      (if (not (`self.CharacterSelected`))
        (bind _output_get (set `self.CharacterIndexValue` (+ (`self.CharacterIndexValue`) 1)))
        (if (> _output_get 1)
          (bind _output_get_2 (set `self.CharacterIndexValue` 0)))
        (`self.Set Character Mesh` _output_get_2 true)
        (bind _output_get_3 (set `self.HairIndexValue` (`KismetMathLibrary.RandomInteger` 7)))
        (bind _output_get_4 (set `self.BodyIndexValue` (`KismetMathLibrary.RandomInteger` 4)))
        (`self.Set Hair Material` _output_get_3)
        (`self.Set Body Material` _output_get_4 (`self.CharacterIndexValue`))
        (bind _output_get_5 (set `self.HairIndexValue` (`KismetMathLibrary.RandomInteger` 7) :!label _label_2))
        (bind _output_get_6 (set `self.BodyIndexValue` (`KismetMathLibrary.RandomInteger` 4)))
        (`self.Set Hair Material` _output_get_5)
        (`self.Set Body Material` _output_get_6 (`self.CharacterIndexValue`))
        (goto _label))
      (elif (< AxisValue -0.3)
        (if (not (`self.CharacterSelected`))
          (bind _output_get_7 (set `self.CharacterIndexValue` (- (`self.CharacterIndexValue`) 1)))
          (if (< _output_get_7 0)
            (bind _output_get_8 (set `self.CharacterIndexValue` 1)))
          (`self.Set Character Mesh` _output_get_8 true)
          (bind _output_get_9 (set `self.HairIndexValue` (`KismetMathLibrary.RandomInteger` 7)))
          (bind _output_get_10 (set `self.BodyIndexValue` (`KismetMathLibrary.RandomInteger` 4)))
          (`self.Set Hair Material` _output_get_9)
          (`self.Set Body Material` _output_get_10 (`self.CharacterIndexValue`))
          (goto _label_2))))))

(fn `AssignMeshObjects`
  (bind _skeletalmesh (`self.SkeletalMesh`))
  (`StaticMeshComponent.SetStaticMesh` (`self.R_Shoe`) "/Game/Assets/Models/Environments/Characters/Ruth/shoe2.shoe2")
  (`StaticMeshComponent.SetStaticMesh` (`self.L_Shoe`) "/Game/Assets/Models/Environments/Characters/Ruth/shoe2.shoe2")
  (`StaticMeshComponent.SetStaticMesh` (`self.Dress`) "/Game/Assets/Models/Accesories/Ruth_Dress_THIS_ONE_.Ruth_Dress_THIS_ONE_")
  (`StaticMeshComponent.SetStaticMesh` (`self.Hair`) "/Game/Assets/Models/Accesories/Ruth_hair__2_.Ruth_hair__2_")
  (`SkinnedMeshComponent.SetSkinnedAssetAndUpdate` _skeletalmesh "/Game/Assets/Models/Environments/Characters/Ruth/Real_Ruth_UE4.Real_Ruth_UE4" true)
  (`SkeletalMeshComponent.SetAnimationMode` _skeletalmesh "AnimationSingleNode")
  (`SkeletalMeshComponent.PlayAnimation` _skeletalmesh "/Game/Assets/Animations/Ruth/Ruth_Idle_Anim.Ruth_Idle_Anim" true)
  (`PrimitiveComponent.SetMaterial` _skeletalmesh 2 "/Game/Assets/Material/Characters/Ruth/ruthFace.ruthFace"))

(fn `Set Body Material`
  (params (ColourID :type Integer) (CharacterID :type Integer))
  (bind _dress (`self.Dress`))
  (bind _skeletalmesh (`self.SkeletalMesh`))
  (bind _skeletalmesh_2 (`self.SkeletalMesh`))
  (switch `int` CharacterID
    (:`0`
      (switch `int` ColourID
        (:`Default`
          _)
        (:`0`
          (`PrimitiveComponent.SetMaterial` _skeletalmesh_2 1 "/Game/Assets/Material/Characters/Ruth/RedI.RedI")
          (`PrimitiveComponent.SetMaterial` _dress 0 "/Game/Assets/Material/Characters/Ruth/RedI.RedI"))
        (:`1`
          (`PrimitiveComponent.SetMaterial` _skeletalmesh_2 1 "/Game/Assets/Material/Characters/Ruth/Blue.Blue")
          (`PrimitiveComponent.SetMaterial` _dress 0 "/Game/Assets/Material/Characters/Ruth/Blue.Blue"))
        (:`2`
          (`PrimitiveComponent.SetMaterial` _skeletalmesh_2 1 "/Game/Assets/Material/Characters/Ruth/Green.Green")
          (`PrimitiveComponent.SetMaterial` _dress 0 "/Game/Assets/Material/Characters/Ruth/Green.Green"))
        (:`3`
          (`PrimitiveComponent.SetMaterial` _skeletalmesh_2 1 "/Game/Assets/Material/Characters/Ruth/Yellow.Yellow")
          (`PrimitiveComponent.SetMaterial` _dress 0 "/Game/Assets/Material/Characters/Ruth/Yellow.Yellow"))
        (:`4`
          (`PrimitiveComponent.SetMaterial` _skeletalmesh_2 1 "/Game/Assets/Material/Characters/Ruth/Purple.Purple")
          (`PrimitiveComponent.SetMaterial` _dress 0 "/Game/Assets/Material/Characters/Ruth/Purple.Purple")))
      (`PrimitiveComponent.SetMaterial` _skeletalmesh_2 2 "/Game/Assets/Material/Characters/Ruth/ruthFace.ruthFace"))
    (:`1`
      (switch `int` ColourID
        (:`0`
          (`PrimitiveComponent.SetMaterial` _skeletalmesh 2 "/Game/Assets/Material/Characters/Aeiou/AEIOU_RedLimbs_Mat.AEIOU_RedLimbs_Mat"))
        (:`1`
          (`PrimitiveComponent.SetMaterial` _skeletalmesh 2 "/Game/Assets/Material/Characters/Aeiou/AEIOU_BlueLimbs_Mat.AEIOU_BlueLimbs_Mat"))
        (:`2`
          (`PrimitiveComponent.SetMaterial` _skeletalmesh 2 "/Game/Assets/Material/Characters/Aeiou/AEIOU_GreenLimbs_Mat.AEIOU_GreenLimbs_Mat"))
        (:`3`
          (`PrimitiveComponent.SetMaterial` _skeletalmesh 2 "/Game/Assets/Material/Characters/Aeiou/AEIOU_YellowLimbs_Mat.AEIOU_YellowLimbs_Mat"))
        (:`4`
          (`PrimitiveComponent.SetMaterial` _skeletalmesh 2 "/Game/Assets/Material/Characters/Aeiou/AEIOU_PurpleLimbs_Mat.AEIOU_PurpleLimbs_Mat")))
      (`PrimitiveComponent.SetMaterial` _skeletalmesh_2 1 "/Game/Assets/Material/Characters/Aeiou/AEIOUBodyText.AEIOUBodyText"))))

(fn `Set Character Mesh`
  (params (`Character Index` :type Integer) (`Connected to game` :type Boolean))
  (bind _skeletalmesh (`self.SkeletalMesh`))
  (bind _hair (`self.Hair`))
  (bind _dress (`self.Dress`))
  (bind _l_shoe (`self.L_Shoe`))
  (bind _r_shoe (`self.R_Shoe`))
  (if `Connected to game`
    (switch `int` `Character Index`
      (:`0`
        (`SkinnedMeshComponent.SetSkinnedAssetAndUpdate` _skeletalmesh "/Game/Assets/Models/Environments/Characters/Ruth/Real_Ruth_UE4.Real_Ruth_UE4" true)
        (`SkeletalMeshComponent.SetAnimationMode` _skeletalmesh "AnimationSingleNode")
        (`SkeletalMeshComponent.PlayAnimation` _skeletalmesh "/Game/Assets/Animations/Ruth/Ruth_Idle_Anim.Ruth_Idle_Anim" true)
        (`StaticMeshComponent.SetStaticMesh` _hair "/Game/Assets/Models/Accesories/Ruth_hair__2_.Ruth_hair__2_")
        (`StaticMeshComponent.SetStaticMesh` _dress "/Game/Assets/Models/Accesories/Ruth_Dress_THIS_ONE_.Ruth_Dress_THIS_ONE_")
        (`StaticMeshComponent.SetStaticMesh` _l_shoe "/Game/Assets/Models/Environments/Characters/Ruth/shoe2.shoe2")
        (`StaticMeshComponent.SetStaticMesh` _r_shoe "/Game/Assets/Models/Environments/Characters/Ruth/shoe2.shoe2"))
      (:`1`
        (`SkinnedMeshComponent.SetSkinnedAssetAndUpdate` _skeletalmesh "/Game/Assets/Models/Environments/Characters/AEIOU/UE4_Aeiou.UE4_Aeiou" true)
        (`SkeletalMeshComponent.SetAnimationMode` _skeletalmesh "AnimationSingleNode")
        (`SkeletalMeshComponent.PlayAnimation` _skeletalmesh "/Game/Assets/Animations/AEIOU/Aeiou_Idle.Aeiou_Idle" true)
        (`StaticMeshComponent.SetStaticMesh` _hair null)
        (`StaticMeshComponent.SetStaticMesh` _hair null :!label _label)
        (`StaticMeshComponent.SetStaticMesh` _dress null)
        (`StaticMeshComponent.SetStaticMesh` _l_shoe null)
        (`StaticMeshComponent.SetStaticMesh` _r_shoe null)))
    (else
      (`SkinnedMeshComponent.SetSkinnedAssetAndUpdate` _skeletalmesh null true)
      (`SkeletalMeshComponent.SetAnimationMode` _skeletalmesh "AnimationSingleNode")
      (`SkeletalMeshComponent.PlayAnimation` _skeletalmesh null true)
      (goto _label))))

(fn `Set Hair Material`
  (params (ColourID :type Integer))
  (bind _hair (`self.Hair`))
  (switch `int` ColourID
    (:`0`
      (`PrimitiveComponent.SetMaterial` _hair 0 "/Game/Assets/Material/Characters/Ruth/RedI.RedI")
      (`PrimitiveComponent.SetMaterial` (`self.L_Shoe`) 0 "/Game/Assets/Material/Characters/Ruth/RedI.RedI")
      (`PrimitiveComponent.SetMaterial` (`self.R_Shoe`) 0 "/Game/Assets/Material/Characters/Ruth/RedI.RedI"))
    (:`1`
      (`PrimitiveComponent.SetMaterial` _hair 0 "/Game/Assets/Material/Characters/Ruth/Blue.Blue")
      (`PrimitiveComponent.SetMaterial` (`self.L_Shoe`) 0 "/Game/Assets/Material/Characters/Ruth/Blue.Blue")
      (`PrimitiveComponent.SetMaterial` (`self.R_Shoe`) 0 "/Game/Assets/Material/Characters/Ruth/Blue.Blue"))
    (:`2`
      (`PrimitiveComponent.SetMaterial` _hair 0 "/Game/Assets/Material/Characters/Ruth/Green.Green")
      (`PrimitiveComponent.SetMaterial` (`self.L_Shoe`) 0 "/Game/Assets/Material/Characters/Ruth/Green.Green")
      (`PrimitiveComponent.SetMaterial` (`self.R_Shoe`) 0 "/Game/Assets/Material/Characters/Ruth/Green.Green"))
    (:`3`
      (`PrimitiveComponent.SetMaterial` _hair 0 "/Game/Assets/Material/Characters/Ruth/Yellow.Yellow")
      (`PrimitiveComponent.SetMaterial` (`self.R_Shoe`) 0 "/Game/Assets/Material/Characters/Ruth/Yellow.Yellow")
      (`PrimitiveComponent.SetMaterial` (`self.L_Shoe`) 0 "/Game/Assets/Material/Characters/Ruth/Yellow.Yellow"))
    (:`4`
      (`PrimitiveComponent.SetMaterial` _hair 0 "/Game/Assets/Material/Characters/Ruth/Purple.Purple")
      (`PrimitiveComponent.SetMaterial` (`self.R_Shoe`) 0 "/Game/Assets/Material/Characters/Ruth/Purple.Purple")
      (`PrimitiveComponent.SetMaterial` (`self.L_Shoe`) 0 "/Game/Assets/Material/Characters/Ruth/Purple.Purple"))
    (:`5`
      (`PrimitiveComponent.SetMaterial` _hair 0 "/Game/Assets/Material/Characters/Ruth/Brown.Brown")
      (`PrimitiveComponent.SetMaterial` (`self.R_Shoe`) 0 "/Game/Assets/Material/Characters/Ruth/Brown.Brown")
      (`PrimitiveComponent.SetMaterial` (`self.L_Shoe`) 0 "/Game/Assets/Material/Characters/Ruth/Brown.Brown"))
    (:`6`
      (`PrimitiveComponent.SetMaterial` _hair 0 "/Game/Assets/Material/Characters/Ruth/Black.Black")
      (`PrimitiveComponent.SetMaterial` (`self.R_Shoe`) 0 "/Game/Assets/Material/Characters/Ruth/Black.Black")
      (`PrimitiveComponent.SetMaterial` (`self.L_Shoe`) 0 "/Game/Assets/Material/Characters/Ruth/Black.Black"))
    (:`7`
      (`PrimitiveComponent.SetMaterial` _hair 0 "/Game/Assets/Material/Characters/Ruth/Orange.Orange")
      (`PrimitiveComponent.SetMaterial` (`self.R_Shoe`) 0 "/Game/Assets/Material/Characters/Ruth/Orange.Orange")
      (`PrimitiveComponent.SetMaterial` (`self.L_Shoe`) 0 "/Game/Assets/Material/Characters/Ruth/Orange.Orange"))))

(fn `UnassignMeshObjects`
  (`StaticMeshComponent.SetStaticMesh` (`self.R_Shoe`) null)
  (`StaticMeshComponent.SetStaticMesh` (`self.L_Shoe`) null)
  (`StaticMeshComponent.SetStaticMesh` (`self.Dress`) null)
  (`StaticMeshComponent.SetStaticMesh` (`self.Hair`) null)
  (`SkinnedMeshComponent.SetSkinnedAssetAndUpdate` (`self.SkeletalMesh`) null true))

(fn `UserConstructionScript`)
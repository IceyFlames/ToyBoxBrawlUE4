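; MapSelectPawn is the input pawn for a map selection screen that chooses between the GreyboxPool and Lab levels.
; On BeginPlay it finds the existing SelectMap widget and caches it.
; D-pad presses and the MoveRight axis step a wrapping MapSelected index and update the widget highlight, with a Delay throttling stick input past a dead zone.
; The bottom button opens the level matching the current index.
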(event `self.ReceiveBeginPlay`
  (bind _foundwidgets (`WidgetBlueprintLibrary.GetAllWidgetsOfClass` "/Game/Blueprints/Widgets/SelectMap.SelectMap_C"))
  (set `self.SelectMap` (cast `/Game/Blueprints/Widgets/SelectMap` (`KismetArrayLibrary.Array_Get` _foundwidgets) :!pure true)))

(event `InputAction|Dpad_left`
  (params (Key :type "Key Structure" :default "AnyKey"))
  (bind _mapselected (`self.MapSelected`))
  (:`Pressed`
    (set `self.MapSelected` (- _mapselected 1))
    (if (< _mapselected 0)
      (set `self.MapSelected` 1))
    (`/Game/Blueprints/Widgets/SelectMap.MapHighlighted` (`self.SelectMap`) _mapselected :!label _label)))

(event `InputAction|Dpad_right`
  (params (Key :type "Key Structure" :default "AnyKey"))
  (bind _mapselected (`self.MapSelected`))
  (:`Pressed`
    (set `self.MapSelected` (+ _mapselected 1))
    (if (> _mapselected 1)
      (set `self.MapSelected` 0)
      (goto _label)
      (else
        (goto _label)))))

(event `InputAction|Bottom_Button`
  (params (Key :type "Key Structure" :default "AnyKey"))
  (:`Pressed`
    (switch `int` (`self.MapSelected`)
      (:`0`
        (`GameplayStatics.OpenLevel` "GreyboxPool"))
      (:`1`
        (`GameplayStatics.OpenLevel` "Lab")))))

(event `InputAxis|MoveRight`
  (params (AxisValue :type "Float (single-precision)"))
  (bind _mapselected (`self.MapSelected`))
  (bind _returnvalue (- _mapselected 1))
  (`KismetSystemLibrary.Delay` 0.3)
  (if (< AxisValue -0.15)
    (set `self.MapSelected` _returnvalue)
    (if (< _returnvalue -1)
      (set `self.MapSelected` 1))
    (`/Game/Blueprints/Widgets/SelectMap.MapHighlighted` (`self.SelectMap`) (stale _output_get) :!label _label_2)
    (elif (> AxisValue 0.15)
      (bind _output_get (set `self.MapSelected` (+ _mapselected 1)))
      (if (> _output_get 1)
        (set `self.MapSelected` 0)
        (goto _label_2)
        (else
          (goto _label_2))))))

(fn `UserConstructionScript`)
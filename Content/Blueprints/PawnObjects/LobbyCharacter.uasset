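; Lobby pawn that lets a controller's player join and customise a character (Ruth or AEIOU) before a match.
; Boolean flags step through join, character, hair colour (skipped for AEIOU) and body colour, with face buttons confirming or backing out.
; D-pad and delayed stick input cycle options, updating preview meshes, materials and the JoinLobby widget.
; Confirming adds a player struct to GameInfo's TPlayers; Pause's level start is unwired.
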(event `InputAction|Pause`
  (params (Key :type "Key Structure" :default "AnyKey"))
  ;[1 1 1] Start is Pressed to initiate game
  (:`Pressed`
    (if (and (`self.HairColourSelected`) (> (`KismetArrayLibrary.Array_Length` (`GameInstanceTBB._TPlayers` (cast `/Game/Blueprints/GameInstance/GameInfo` (`GameplayStatics.GetGameInstance`) :!pure true))) 1))
      _)))

(event `InputAction|Bottom_Button`
  (params (Key :type "Key Structure" :default "AnyKey"))
  (bind _hairindexvalue (`self.HairIndexValue`))
  ;[0.08708 0 1] Selecting Options
  (:`Pressed`
    (if (`self.ConnectedtoGame`)
      (if (`self.CharacterSelected`)
        (if (`self.HairColourSelected`)
          (if (not (`self.SwimSuitSelected`))
            (set `self.SwimSuitSelected` true)
            (`/Game/Blueprints/Widgets/JoinLobby.SetReadyTextVisible` (cast `/Game/Blueprints/Widgets/JoinLobby` (`KismetArrayLibrary.Array_Get` (stale `InputAction|Bottom_Button` _foundwidgets)) :!pure true) (`self.ControllerID`) true)
            (switch `int` (`self.CharacterIndexValue`)
              (:`0`
                (set `self.CharacterName` "Ruth"))
              (:`1`
                (set `self.CharacterName` "AEIOU"))
              (:`2`
                (bind _output_get (set `self.CharacterName` "Ruth"))))
            (bind _output_get_2 (set `self.PlayerStructure` (make `PlayerCharacter` (`self.ControllerID`) _output_get (`self.BodyIndexValue`) _hairindexvalue)))
            (`KismetArrayLibrary.Array_AddUnique` (`GameInstanceTBB._TPlayers` (cast `/Game/Blueprints/GameInstance/GameInfo` (`GameplayStatics.GetGameInstance`) :!pure true)) _output_get_2))
          (else
            (set `self.HairColourSelected` true)))
        (else
          (set `self.CharacterSelected` true)
          (switch `int` (`self.CharacterIndexValue`)
            (:`1`
              (set `self.HairColourSelected` true)))))
      (else
        (set `self.ConnectedtoGame` true)
        (bind _foundwidgets (`WidgetBlueprintLibrary.GetAllWidgetsOfClass` "/Game/Blueprints/Widgets/JoinLobby.JoinLobby_C"))
        (`self.AssignMeshObjects`)
        (`self.Set Hair Material` _hairindexvalue)))))

(event `InputAction|Right_button`
  (params (Key :type "Key Structure" :default "AnyKey"))
  ;[0.08708 0 1] Selecting Options
  (:`Pressed`
    (if (`self.HairColourSelected`)
      (set `self.HairColourSelected` false)
      (`/Game/Blueprints/Widgets/JoinLobby.SetReadyTextVisible` (cast `/Game/Blueprints/Widgets/JoinLobby` (`KismetArrayLibrary.Array_Get` (stale `InputAction|Bottom_Button` _foundwidgets)) :!pure true) (`self.ControllerID`) false)
      (`KismetArrayLibrary.Array_RemoveItem` (`GameInstanceTBB._TPlayers` (cast `/Game/Blueprints/GameInstance/GameInfo` (`GameplayStatics.GetGameInstance`) :!pure true)) (`self.PlayerStructure`))
      (elif (`self.SwimSuitSelected`)
        (set `self.SwimSuitSelected` false)
        (elif (`self.CharacterSelected`)
          (set `self.CharacterSelected` false)
          (elif (`self.ConnectedtoGame`)
            (set `self.ConnectedtoGame` false)))))))

(event `InputAction|Dpad_up`
  (params (Key :type "Key Structure" :default "AnyKey"))
  (bind _controllerid (`self.ControllerID`))
  (bind _characterindexvalue (`self.CharacterIndexValue`))
  ;[1 0.4152 0] Dpad Up Input
  (:`Pressed`
    (if (`self.ConnectedtoGame`)
      (if (`self.CharacterSelected`)
        (if (`self.HairColourSelected`)
          (if (not (`self.SwimSuitSelected`))
            (bind _output_get (set `self.BodyIndexValue` (+ (`self.BodyIndexValue`) 1)))
            (if (> _output_get 4)
              (bind _output_get_2 (set `self.BodyIndexValue` 0)))
            (bind _asjoin_lobby (cast `/Game/Blueprints/Widgets/JoinLobby` (`KismetArrayLibrary.Array_Get` (stale `InputAction|Bottom_Button` _foundwidgets)) :!pure true))
            (`/Game/Blueprints/Widgets/JoinLobby.SetTorsoColourUI` _asjoin_lobby _controllerid _output_get)
            (`self.Set Body Material` _output_get_2 (stale _output_get_6)))
          (else
            (bind _output_get_3 (set `self.HairIndexValue` (+ (`self.HairIndexValue`) 1)))
            (if (> _output_get_3 7)
              (bind _output_get_4 (set `self.HairIndexValue` 0)))
            (`/Game/Blueprints/Widgets/JoinLobby.SetHairColourUI` _asjoin_lobby _controllerid _output_get_4)
            (`self.Set Hair Material` _output_get_4)))
        (else
          (bind _output_get_5 (set `self.CharacterIndexValue` (+ _characterindexvalue 1)))
          (if (> _output_get_5 1)
            (bind _output_get_6 (set `self.CharacterIndexValue` 0)))
          (`self.Set Character Mesh` _output_get_6 true)))
      (else
        (`self.Set Character Mesh` _characterindexvalue)))))

(event `InputAction|Dpad_down`
  (params (Key :type "Key Structure" :default "AnyKey"))
  (bind _controllerid (`self.ControllerID`))
  (bind _characterindexvalue (`self.CharacterIndexValue`))
  ;[0.7913 0.016 1] DpadDown Input
  (:`Pressed`
    (if (`self.ConnectedtoGame`)
      (if (`self.CharacterSelected`)
        (if (`self.HairColourSelected`)
          (if (not (`self.SwimSuitSelected`))
            (bind _output_get (set `self.BodyIndexValue` (- (`self.BodyIndexValue`) 1)))
            (if (< _output_get 0)
              (bind _output_get_2 (set `self.BodyIndexValue` 4)))
            (bind _asjoin_lobby (cast `/Game/Blueprints/Widgets/JoinLobby` (`KismetArrayLibrary.Array_Get` (stale `InputAction|Bottom_Button` _foundwidgets)) :!pure true))
            (`/Game/Blueprints/Widgets/JoinLobby.SetTorsoColourUI` _asjoin_lobby _controllerid _output_get_2)
            (`self.Set Body Material` _output_get_2 (stale _output_get_6)))
          (else
            (bind _output_get_3 (set `self.HairIndexValue` (- (`self.HairIndexValue`) 1)))
            (if (< _output_get_3 0)
              (bind _output_get_4 (set `self.HairIndexValue` 7)))
            (`/Game/Blueprints/Widgets/JoinLobby.SetHairColourUI` _asjoin_lobby _controllerid _output_get_4)
            (`self.Set Hair Material` _output_get_4)))
        (else
          (bind _output_get_5 (set `self.CharacterIndexValue` (- _characterindexvalue 1)))
          (if (< _output_get_5 0)
            (bind _output_get_6 (set `self.CharacterIndexValue` 1)))
          (`self.Set Character Mesh` _output_get_6 true)))
      (else
        (`self.Set Character Mesh` _characterindexvalue)))))

(event `InputAxis|MoveForward`
  (params (AxisValue :type "Float (single-precision)"))
  (bind _controllerid (`self.ControllerID`))
  (bind _controllerid_2 (`self.ControllerID`))
  ;[1 1 1] Analog Stick Support
  (`KismetSystemLibrary.Delay` 0.15)
  (if (> AxisValue 0.3)
    (if (`self.CharacterSelected`)
      (if (`self.HairColourSelected`)
        (if (not (`self.SwimSuitSelected`))
          (bind _output_get (set `self.BodyIndexValue` (+ (`self.BodyIndexValue`) 1)))
          (if (> _output_get 7)
            (bind _output_get_2 (set `self.BodyIndexValue` 0)))
          (bind _asjoin_lobby (cast `/Game/Blueprints/Widgets/JoinLobby` (`KismetArrayLibrary.Array_Get` (stale `InputAction|Bottom_Button` _foundwidgets)) :!pure true))
          (`/Game/Blueprints/Widgets/JoinLobby.SetTorsoColourUI` _asjoin_lobby _controllerid _output_get)
          (`self.Set Body Material` _output_get_2 (stale _output_get_6)))
        (else
          (bind _output_get_3 (set `self.HairIndexValue` (+ (`self.HairIndexValue`) 1)))
          (if (> _output_get_3 7)
            (bind _output_get_4 (set `self.HairIndexValue` 0)))
          (`/Game/Blueprints/Widgets/JoinLobby.SetHairColourUI` _asjoin_lobby _controllerid _output_get_4)
          (`self.Set Hair Material` _output_get_4)))
      (else
        (bind _output_get_5 (set `self.CharacterIndexValue` (+ (`self.CharacterIndexValue`) 1)))
        (if (> _output_get_5 1)
          (bind _output_get_6 (set `self.CharacterIndexValue` 0)))
        (`self.Set Character Mesh` _output_get_6 true)))
    (elif (< AxisValue -0.3)
      (if (`self.CharacterSelected`)
        (if (`self.HairColourSelected`)
          (if (not (`self.SwimSuitSelected`))
            (bind _output_get_7 (set `self.BodyIndexValue` (- (`self.BodyIndexValue`) 1)))
            (if (< _output_get_7 0)
              (bind _output_get_8 (set `self.BodyIndexValue` 4)))
            (`/Game/Blueprints/Widgets/JoinLobby.SetTorsoColourUI` _asjoin_lobby _controllerid_2 _output_get_8)
            (`self.Set Body Material` _output_get_8 (stale _output_get_12)))
          (else
            (bind _output_get_9 (set `self.HairIndexValue` (- (`self.HairIndexValue`) 1)))
            (if (< _output_get_9 0)
              (bind _output_get_10 (set `self.HairIndexValue` 7)))
            (`/Game/Blueprints/Widgets/JoinLobby.SetHairColourUI` _asjoin_lobby _controllerid_2 _output_get_10)
            (`self.Set Hair Material` _output_get_10)))
        (else
          (bind _output_get_11 (set `self.CharacterIndexValue` (- (`self.CharacterIndexValue`) 1)))
          (if (< _output_get_11 0)
            (bind _output_get_12 (set `self.CharacterIndexValue` 1)))
          (`self.Set Character Mesh` _output_get_12 true))))))

(fn `AssignMeshObjects`
  (bind _skeletalmesh (`self.SkeletalMesh`))
  (`StaticMeshComponent.SetStaticMesh` (`self.Hair`) "/Game/Assets/Models/Accesories/Ruth_hair__2_.Ruth_hair__2_")
  (`SkinnedMeshComponent.SetSkinnedAssetAndUpdate` _skeletalmesh "/Game/Assets/Models/Characters/Ruth/Real_Ruth_UE4.Real_Ruth_UE4" true)
  (`SkeletalMeshComponent.SetAnimationMode` _skeletalmesh "AnimationSingleNode")
  (`SkeletalMeshComponent.PlayAnimation` _skeletalmesh "/Game/Assets/Animations/Ruth/Ruth_Idle_Anim.Ruth_Idle_Anim" true))

(fn `Set Body Material`
  (params (ColourID :type Integer) (CharacterID :type Integer))
  (bind _skeletalmesh (`self.SkeletalMesh`))
  (bind _skeletalmesh_2 (`self.SkeletalMesh`))
  (switch `int` CharacterID
    (:`0`
      (switch `int` ColourID
        (:`0`
          (`PrimitiveComponent.SetMaterial` _skeletalmesh_2 1 "/Game/Assets/Material/Characters/Ruth/RedI.RedI"))
        (:`1`
          (`PrimitiveComponent.SetMaterial` _skeletalmesh_2 1 "/Game/Assets/Material/Characters/Ruth/Blue.Blue"))
        (:`2`
          (`PrimitiveComponent.SetMaterial` _skeletalmesh_2 1 "/Game/Assets/Material/Characters/Ruth/Green.Green"))
        (:`3`
          (`PrimitiveComponent.SetMaterial` _skeletalmesh_2 1 "/Game/Assets/Material/Characters/Ruth/Yellow.Yellow"))
        (:`4`
          (`PrimitiveComponent.SetMaterial` _skeletalmesh_2 1 "/Game/Assets/Material/Characters/Ruth/Purple.Purple")))
      (`PrimitiveComponent.SetMaterial` _skeletalmesh_2 2 "/Game/Assets/Material/Characters/Ruth/ruthFace.ruthFace"))
    (:`1`
      (switch `int` ColourID
        (:`0`
          (`PrimitiveComponent.SetMaterial` _skeletalmesh 2 "/Game/Assets/Material/Characters/Aeiou/AEIOU_RedLimbs_Mat.AEIOU_RedLimbs_Mat"))
        (:`1`
          (`PrimitiveComponent.SetMaterial` _skeletalmesh 2 "/Game/Assets/Material/Characters/Aeiou/AEIOU_BlueLimbs_Mat.AEIOU_BlueLimbs_Mat"))
        (:`2`
          (`PrimitiveComponent.SetMaterial` _skeletalmesh 2 "/Game/Assets/Material/Characters/Aeiou/AEIOU_GreenLimbs_Mat.AEIOU_GreenLimbs_Mat"))
        (:`3`
          (`PrimitiveComponent.SetMaterial` _skeletalmesh 2 "/Game/Assets/Material/Characters/Aeiou/AEIOU_YellowLimbs_Mat.AEIOU_YellowLimbs_Mat"))
        (:`4`
          (`PrimitiveComponent.SetMaterial` _skeletalmesh 2 "/Game/Assets/Material/Characters/Aeiou/AEIOU_PurpleLimbs_Mat.AEIOU_PurpleLimbs_Mat"))))))

(fn `Set Character Mesh`
  (params (`Character Index` :type Integer) (`Connected to game` :type Boolean))
  (bind _skeletalmesh (`self.SkeletalMesh`))
  (bind _hair (`self.Hair`))
  (if `Connected to game`
    (switch `int` `Character Index`
      (:`0`
        (`SkinnedMeshComponent.SetSkinnedAssetAndUpdate` _skeletalmesh "/Game/Assets/Models/Characters/Ruth/Real_Ruth_UE4.Real_Ruth_UE4" true)
        (`SkeletalMeshComponent.SetAnimationMode` _skeletalmesh "AnimationSingleNode")
        (`SkeletalMeshComponent.PlayAnimation` _skeletalmesh "/Game/Assets/Animations/Ruth/Ruth_Idle_Anim.Ruth_Idle_Anim" true)
        (`StaticMeshComponent.SetStaticMesh` _hair "/Game/Assets/Models/Accesories/Ruth_hair__2_.Ruth_hair__2_"))
      (:`1`
        (`SkinnedMeshComponent.SetSkinnedAssetAndUpdate` _skeletalmesh "/Game/Assets/Models/Characters/AEIOU/UE4_Aeiou.UE4_Aeiou" true)
        (`SkeletalMeshComponent.SetAnimationMode` _skeletalmesh "AnimationSingleNode")
        (`SkeletalMeshComponent.PlayAnimation` _skeletalmesh "/Game/Assets/Animations/AEIOU/Aeiou_Idle.Aeiou_Idle" true)
        (`StaticMeshComponent.SetStaticMesh` _hair null)))
    (else
      (`SkinnedMeshComponent.SetSkinnedAssetAndUpdate` _skeletalmesh null true)
      (`SkeletalMeshComponent.SetAnimationMode` _skeletalmesh "AnimationSingleNode")
      (`SkeletalMeshComponent.PlayAnimation` _skeletalmesh null true)
      (`StaticMeshComponent.SetStaticMesh` _hair null))))

(fn `Set Hair Material`
  (params (ColourID :type Integer))
  (bind _hair (`self.Hair`))
  (switch `int` ColourID
    (:`0`
      (`PrimitiveComponent.SetMaterial` _hair 0 "/Game/Assets/Material/Characters/Ruth/RedI.RedI"))
    (:`1`
      (`PrimitiveComponent.SetMaterial` _hair 0 "/Game/Assets/Material/Characters/Ruth/Blue.Blue"))
    (:`2`
      (`PrimitiveComponent.SetMaterial` _hair 0 "/Game/Assets/Material/Characters/Ruth/Green.Green"))
    (:`3`
      (`PrimitiveComponent.SetMaterial` _hair 0 "/Game/Assets/Material/Characters/Ruth/Yellow.Yellow"))
    (:`4`
      (`PrimitiveComponent.SetMaterial` _hair 0 "/Game/Assets/Material/Characters/Ruth/Purple.Purple"))
    (:`5`
      (`PrimitiveComponent.SetMaterial` _hair 0 "/Game/Assets/Material/Characters/Ruth/Brown.Brown"))
    (:`6`
      (`PrimitiveComponent.SetMaterial` _hair 0 "/Game/Assets/Material/Characters/Ruth/Black.Black"))
    (:`7`
      (`PrimitiveComponent.SetMaterial` _hair 0 "/Game/Assets/Material/Characters/Ruth/Orange.Orange"))))

(fn `UserConstructionScript`)
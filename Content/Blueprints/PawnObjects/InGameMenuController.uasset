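; In-game menu controller object that shows InGameMenuWidget and handles gamepad navigation through its four options.
; D-pad and MoveForward axis input move a wrapping selection index that recolours the widget's highlighted button, with a short Delay pacing analog scrolling.
; The bottom button passes the selection to the widget's ConfirmOption.
; For the first option, it also makes the player controller possess the character stored through PossessCharacterReference.
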(event `self.ReceiveBeginPlay`
  ;[1 1 1] BeginPlay Stuffs
  (bind _returnvalue (`|CreateWidget` "/Game/Blueprints/Widgets/InGameMenuWidget.InGameMenuWidget_C"))
  (bind _output_get (set `self.Widget` _returnvalue))
  (`UserWidget.AddToViewport` _returnvalue 0)
  (`UserWidget.AddToViewport` _output_get 0)
  (`/Game/Blueprints/Widgets/InGameMenuWidget.SetButtonColour` _returnvalue (`self.ButtonSelected`) (struct :`G` 1.0 :`B` 0.034785 :`A` 1.0))
  (`/Game/Blueprints/Widgets/InGameMenuWidget.SetButtonColour` _output_get (`self.ButtonSelected`) (struct :`G` 1.0 :`B` 0.034785 :`A` 1.0)))

(event `InputAction|Dpad_up`
  (params (Key :type "Key Structure" :default "AnyKey"))
  ;[0.2546 0.114 1] Selecting which button is highlighted
  (:`Pressed`
    (bind _result (`/Engine/EditorBlueprintResources/StandardMacros.DecrementInt` (`self.ButtonSelected`))
      (:`  `
        (if (< _result 0)
          (bind _output_get (set `self.ButtonSelected` 3)))
        (`/Game/Blueprints/Widgets/InGameMenuWidget.SetButtonColour` (`self.Widget`) _output_get (struct :`G` 1.0 :`A` 1.0) :!label _label)))))

(event `InputAction|Dpad_down`
  (params (Key :type "Key Structure" :default "AnyKey"))
  ;[0.2546 0.114 1] Selecting which button is highlighted
  (:`Pressed`
    (bind _result (`/Engine/EditorBlueprintResources/StandardMacros.IncrementInt` (`self.ButtonSelected`))
      (:`  `
        (if (> _result 3)
          (set `self.ButtonSelected` 0)
          (goto _label)
          (else
            (goto _label)))))))

(event `InputAction|Bottom_Button`
  (params (Key :type "Key Structure" :default "AnyKey"))
  (bind _buttonselected (`self.ButtonSelected`))
  (:`Pressed`
    (`/Game/Blueprints/Widgets/InGameMenuWidget.ConfirmOption` (`self.Widget`) _buttonselected)
    (if (== _buttonselected 0)
      (`Controller.Possess` (`GameplayStatics.GetPlayerController` (`self.ControllerID`)) (`self.PossessActorRef`)))))

(event `InputAxis|MoveForward`
  (params (AxisValue :type "Float (single-precision)"))
  (bind _buttonselected (`self.ButtonSelected`))
  ;[1 0 0.5417] Analog Support
  (`KismetSystemLibrary.Delay` 0.15)
  (if (> AxisValue 0.3)
    (bind _result (`/Engine/EditorBlueprintResources/StandardMacros.DecrementInt` _buttonselected)
      (:`  `
        (if (< _result 0)
          (set `self.ButtonSelected` 3))))
    (elif (< AxisValue -0.3)
      (bind _result_2 (`/Engine/EditorBlueprintResources/StandardMacros.IncrementInt` _buttonselected)
        (:`  `
          (if (> _result_2 3)
            (bind _output_get (set `self.ButtonSelected` 0)))))))
  (`/Game/Blueprints/Widgets/InGameMenuWidget.SetButtonColour` (`self.Widget`) _output_get (struct :`G` 1.0 :`A` 1.0)))

(fn `PossessCharacterReference`
  (params (Character :type "Pawn Object Reference") (ControllerID :type Integer))
  (set `self.PossessActorRef` Character)
  (set `self.ControllerID` ControllerID))

(fn `UserConstructionScript`)
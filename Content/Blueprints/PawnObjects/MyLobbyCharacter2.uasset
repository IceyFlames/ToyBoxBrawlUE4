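; Lobby character that drives the character-creation UI shown on its widget component.
; BeginPlay stores its body, hair, hat, torso and shoe components as the current parts.
; UpdateWidgets switches CCWidget2 between the clothing selector, highlighting hat, torso or shoe items by CharacterID, and the main HUD, set by CreationID.
; UpdateColorWheel passes visibility and rotation to the widget, with rotation also setting the wheel's colour.
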(event `self.ReceiveBeginPlay`
  (set `self.CurrentMesh` (`self.CharacterMesh`))
  (set `self.CurrentHair` (`self.HairMesh`))
  (set `self.CurrentHat` (`self.HatMesh`))
  (set `self.CurrentTorso` (`self.TorsoMesh`))
  (set `self.CurrentLeftShoe` (`self.LeftShoe`))
  (set `self.CurrentRightShoe` (`self.RightShoe`)))

(event `self.UpdateWidgets`
  (params (_CreationID :type Integer))
  (bind _characterid (`self.CharacterID`))
  (bind _clothingoptionhighlighted (`self.ClothingOptionHighlighted`))
  (bind _asccwidget_2 (cast `/Game/Blueprints/Widgets/CCWidget2` (`WidgetComponent.GetUserWidgetObject` (`self.Widget`)) :!pure true))
  (if (`self.ClothingOptionSelected`)
    (`/Game/Blueprints/Widgets/CCWidget2.DisplayClothingSelectorHUD` _asccwidget_2 _clothingoptionhighlighted true)
    (switch `int` _clothingoptionhighlighted
      (:`0`
        (`/Game/Blueprints/Widgets/CCWidget2.HighlightHatID` _asccwidget_2 _characterid (`self.HatIDHighlighted`)))
      (:`1`
        (`/Game/Blueprints/Widgets/CCWidget2.HighlightTorsoID` _asccwidget_2 _characterid (`self.TorsoIDHightlighted`)))
      (:`3`
        (`/Game/Blueprints/Widgets/CCWidget2.HighShoesID` _asccwidget_2 _characterid (`self.ShoesIDHighlighted`))))
    (else
      (`/Game/Blueprints/Widgets/CCWidget2.DisplayClothingSelectorHUD` _asccwidget_2 0 false)
      (switch `int` _CreationID
        (:`Default`
          (`/Game/Blueprints/Widgets/CCWidget2.DisplayHud` _asccwidget_2 true :!label _label)
          (`/Game/Blueprints/Widgets/CCWidget2.SetClothingOptionOpacity` _asccwidget_2 _CreationID))
        (:`-1`
          (`/Game/Blueprints/Widgets/CCWidget2.DisplayHud` _asccwidget_2 false))
        (:`0`
          (goto _label))
        (:`1`
          (goto _label))))))

(event `self.UpdateColorWheel`
  (params (visble :type Boolean) (rotation :type "Float (single-precision)"))
  (bind _asccwidget_2 (cast `/Game/Blueprints/Widgets/CCWidget2` (`WidgetComponent.GetUserWidgetObject` (`self.Widget`)) :!pure true))
  (`/Game/Blueprints/Widgets/CCWidget2.DisplayColorWheel` _asccwidget_2 visble)
  (`/Game/Blueprints/Widgets/CCWidget2.RotateColorWheel` _asccwidget_2 rotation)
  (`/Game/Blueprints/Widgets/CCWidget2.SetColorWheelColour` _asccwidget_2 rotation))

(fn `UserConstructionScript`)
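; Ruth's character Blueprint, handling limb damage, dismemberment and death; only the right arm's overlap is implemented here, with the other limbs' events left empty.
; A destroying hit hides the arm bone, throws its weapon and calls RagdollEvent, while other hits run a timeline-driven physics blend.
; RagdollEvent acts only when all four limbs are inactive, ragdolling the body, breaking the head joint and incrementing the GameInstance's death count.
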(event `self.ReceiveBeginPlay`
  (set `self.CharacterMesh` (`self.Mesh`)))

(event `self.ReceiveActorBeginOverlap`
  (params (OtherActor :type "Actor Object Reference")))

(event `self.ReceiveTick`
  (params (DeltaSeconds :type "Float (single-precision)")))

(event `self.Lower_LeftLeg.OnComponentBeginOverlap`
  (params (OtherActor :type "Actor Object Reference") (OtherComp :type "PrimitiveComponent Object Reference") (OtherBodyIndex :type Integer) (bFromSweep :type Boolean) (SweepResult :type "HitResult Structure (by ref)")))

(event `self.Lower_RightLeg.OnComponentBeginOverlap`
  (params (OtherActor :type "Actor Object Reference") (OtherComp :type "PrimitiveComponent Object Reference") (OtherBodyIndex :type Integer) (bFromSweep :type Boolean) (SweepResult :type "HitResult Structure (by ref)")))

(event `self.LeftArm.OnComponentBeginOverlap`
  (params (OtherActor :type "Actor Object Reference") (OtherComp :type "PrimitiveComponent Object Reference") (OtherBodyIndex :type Integer) (bFromSweep :type Boolean) (SweepResult :type "HitResult Structure (by ref)")))

(event `self.RightArm.OnComponentBeginOverlap`
  (params (OtherActor :type "Actor Object Reference") (OtherComp :type "PrimitiveComponent Object Reference") (OtherBodyIndex :type Integer) (bFromSweep :type Boolean) (SweepResult :type "HitResult Structure (by ref)"))
  (bind _mesh (`self.Mesh`))
  (bind _righthandlimb (`self.RightHandLimb`))
  (bind (__weapondamage __limbhp __limbactive __bonename) (break `Limb` _righthandlimb))
  ;[1 1 1] Right Arm Takes Damage
  (bind _returnvalue (`self.LimbTakeDamage` OtherActor OtherComp _righthandlimb))
  (if _returnvalue
    (`SkinnedMeshComponent.HideBoneByName` _mesh __bonename "PBO_None")
    (`self.RagdollEvent` (- (`self.K2_GetActorLocation` OtherActor) (`self.K2_GetActorLocation`)))
    (`self.ThrowWeapon` (`self.RightHandWeapon`))
    (`KismetSystemLibrary.Delay` 0.2)
    (set `self.RightHandWeapon` null)
    (else
      (`SkeletalMeshComponent.SetAllBodiesBelowSimulatePhysics` _mesh __bonename false)
      (bind (_direction _physicsblend) (`Timeline|Timeline_0` :!via `PlayFromStart`)
        (:`Update`
          (`SkeletalMeshComponent.SetAllBodiesBelowPhysicsBlendWeight` _mesh __bonename _physicsblend false))))))

(fn `RagdollEvent`
  (params (Force :type "Vector Structure"))
  (bind _mesh (`self.Mesh`))
  (bind _aslevel_info (cast `/Game/Blueprints/GameInstance/LevelInfo` (`GameplayStatics.GetGameInstance`) :!pure true))
  (if (and (not (`self.bLeftArmActive`)) (not (`self.bRightArmActive`)) (not (`self.bLeftLegActive`)) (not (`self.bRightLegActive`)))
    (`PrimitiveComponent.SetSimulatePhysics` _mesh true)
    (`BreakBoneBPLibrary.BoneBreak` _mesh "head_jnt" (0.0 0.0 0.0) Force true)
    (set `/Game/Blueprints/GameInstance/LevelInfo.PlayersDead` (+ (`/Game/Blueprints/GameInstance/LevelInfo.PlayersDead` _aslevel_info) 1) _aslevel_info)))

(fn `ThrowWeapon`
  (params (WeaponReference :type "Actor Object Reference"))
  (bind _asequipment (cast `Equipment` WeaponReference))
  (bind _staticmeshobject (`Equipment.StaticMeshObject` _asequipment))
  (if (`KismetSystemLibrary.IsValid` _staticmeshobject)
    (`PrimitiveComponent.SetSimulatePhysics` _staticmeshobject true)
    (else
      (bind _meshobject (`Equipment.MeshObject` _asequipment))
      (if (`KismetSystemLibrary.IsValid` _meshobject)
        (`PrimitiveComponent.SetSimulatePhysics` _meshobject true))))
  (`self.DetachRootComponentFromParent` true)
  (`Equipment.ObjectThrown` _asequipment)
  (if (== WeaponReference (`self.LeftHandWeapon`))
    (set `self.bLeftArmEquipped` false)
    (else
      (set `self.bRightArmEquipped` false))))

(fn `UserConstructionScript`)